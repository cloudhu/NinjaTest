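; Child actor that makes its parent character's hands reach out and touch nearby objects through hand IK.
; Left and right overlap volumes register objects, then Tick capsule-traces from the character toward each volume for a contact point.
; Timelines blend IK alpha, sent with that point to the AnimInstance.
; Both hands release while falling or interacting, and tracing is skipped in two DYLO movement modes.
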(event `self.ReceiveBeginPlay`
  ;[1 1 1] Begin play sets up owner reference
  (`KismetSystemLibrary.Delay` 0.05)
  (bind _immersive_component (`/Game/ImmersiveTemplate/Blueprints/Library/BPML_IT.BPML Get Immersive Component` (`self.GetParentActor`))
    (:`Is Valid`
      (bind _output_get (set `self.Immersive Component` _immersive_component))
      (bind _output_get_2 (set `self.As Character` (`/Game/ImmersiveTemplate/Blueprints/ImmersiveComponent.REF` _output_get)))
      (bind _dylo_movement_component (`/Game/ImmersiveTemplate/Blueprints/Library/BPML_IT.BPML Get DYLO Movement Component` _output_get_2)
        (:`Is Valid`
          (set `self.DYLO Movement Component` _dylo_movement_component)
          (bind _abp_immersive (`/Game/ImmersiveTemplate/Blueprints/Library/BPML_IT.BPML Get Immersive ABP` (`self.As Character`)))
          (set `self.ABP Immersive` _abp_immersive))))))

(event `self.Right.OnComponentBeginOverlap`
  (params (OverlappedComponent :type "PrimitiveComponent Object Reference") (OtherActor :type "Actor Object Reference") (OtherComp :type "PrimitiveComponent Object Reference") (OtherBodyIndex :type Integer) (bFromSweep :type Boolean) (SweepResult :type "HitResult Structure (by ref)"))
  ;[1 1 1] Right Hand Overlap Start
  (`/Engine/EditorBlueprintResources/StandardMacros.IsValid` OtherActor
    (:`Is Valid`
      (`self.Actor Right`
        (:`then`)
        (:`else`
          (set `self.Actor Right` OtherActor))))))

(event `self.Left.OnComponentBeginOverlap`
  (params (OverlappedComponent :type "PrimitiveComponent Object Reference") (OtherActor :type "Actor Object Reference") (OtherComp :type "PrimitiveComponent Object Reference") (OtherBodyIndex :type Integer) (bFromSweep :type Boolean) (SweepResult :type "HitResult Structure (by ref)"))
  ;[1 1 1] Left Hand Overlap Start
  (`/Engine/EditorBlueprintResources/StandardMacros.IsValid` OtherActor
    (:`Is Valid`
      (`self.Actor Left`
        (:`then`)
        (:`else`
          (set `self.Actor Left` OtherActor))))))

(event `self.ReceiveTick`
  (params (DeltaSeconds :type "Float (single-precision)"))
  (bind _array (`|MakeArray` (`self.As Character`) :!type "Actor Object Reference"))
  ;[1 1 1] Event tick performs trace to see where nearby objects are
  (`self.As Character`
    (:`then`
      (if (`NavMovementComponent.IsFalling` (`Character.CharacterMovement` (`self.As Character`)))
        (`self.Deactivate Left Hand IK` :!label _label)
        (`self.Deactivate Right Hand IK`)
        (elif (`/Game/ImmersiveTemplate/Blueprints/ImmersiveComponent.Is Interacting?` (`self.Immersive Component`))
          (goto _label)
          (else
            (`self.ABP Immersive`
              (:`then`
                (bind _dylo_movement_component (`self.DYLO Movement Component`)
                  (:`then`
                    (bind _movement_mode (`/Game/ImmersiveTemplate/Blueprints/DYLO_MovementComponent.Movement Mode` _dylo_movement_component))
                    (if (not (or (`|EnumEquality` _movement_mode "NewEnumerator2") (`|EnumEquality` _movement_mode "NewEnumerator3")))
                      (`|ExecutionSequence` :!label _label_2
                        (:`then_0`
                          (`self.Actor Left`
                            (:`then`
                              (bind _as_character (`self.As Character`)
                                (:`then`
                                  (bind (_outhit _returnvalue) (`KismetSystemLibrary.CapsuleTraceSingle` (+ (`SceneComponent.K2_GetComponentLocation` (`Character.CapsuleComponent` _as_character)) (0.0 0.0 50.0)) (`SceneComponent.K2_GetComponentLocation` (`self.Left`)) 10.0 30.0 "TraceTypeQuery1" false _array (select `bool` (`self.👾 Debug?`) :`true` "ForOneFrame" :!type "EDrawDebugTrace Enum") false (struct :`G` 0.363356 :`B` 1.0 :`A` 0.25) (struct :`G` 0.118097 :`B` 1.0 :`A` 1.0) 0.2))
                                  (if _returnvalue
                                    (bind (_bblockinghit _binitialoverlap _time _distance _location _impactpoint _normal _impactnormal _physmat _hitactor) (`GameplayStatics.BreakHitResult` _outhit))
                                    (if (not (== _hitactor (`self.Actor Right`)))
                                      (`self.Immersive Component`
                                        (:`then`
                                          (bind _output_get (set `self.Left Hand Location` _impactpoint))
                                          (if (`self.👾 Debug?`)
                                            (`KismetSystemLibrary.DrawDebugSphere` _output_get 2.0 12 (struct :`G` 0.063842 :`B` 1.0 :`A` 1.0) 1.0 1.0))
                                          (`self.Activate Left Hand IK`))
                                        (:`else`)))))
                                (:`else`)))
                            (:`else`)))
                        (:`then_1`
                          (`self.Actor Right`
                            (:`then`
                              (bind _as_character_2 (`self.As Character`)
                                (:`then`
                                  (bind (_outhit_2 _returnvalue_2) (`KismetSystemLibrary.CapsuleTraceSingle` (+ (`SceneComponent.K2_GetComponentLocation` (`Character.CapsuleComponent` _as_character_2)) (0.0 0.0 50.0)) (`SceneComponent.K2_GetComponentLocation` (`self.Right`)) 10.0 30.0 "TraceTypeQuery1" false _array (select `bool` (`self.👾 Debug?`) :`true` "ForOneFrame" :!type "EDrawDebugTrace Enum") false (struct :`R` 1.0 :`B` 0.139431 :`A` 0.25) (struct :`R` 1.0 :`B` 0.101598 :`A` 1.0) 0.2))
                                  (if _returnvalue_2
                                    (bind (_bblockinghit_2 _binitialoverlap_2 _time_2 _distance_2 _location_2 _impactpoint_2 _normal_2 _impactnormal_2 _physmat_2 _hitactor_2) (`GameplayStatics.BreakHitResult` _outhit_2))
                                    (if (not (== _hitactor_2 (`self.Actor Left`)))
                                      (`self.Immersive Component`
                                        (:`then`
                                          (bind _output_get_2 (set `self.Right Hand Location` _impactpoint_2))
                                          (if (`self.👾 Debug?`)
                                            (`KismetSystemLibrary.DrawDebugSphere` _output_get_2 2.0 12 (struct :`R` 1.0 :`B` 0.257036 :`A` 1.0) 1.0 1.0))
                                          (`self.Activate Right Hand IK`))
                                        (:`else`)))))
                                (:`else`)))
                            (:`else`))))))
                  (:`else`
                    (goto _label_2))))
              (:`else`))))))
    (:`else`)))

(event `self.Left.OnComponentEndOverlap`
  (params (OverlappedComponent :type "PrimitiveComponent Object Reference") (OtherActor :type "Actor Object Reference") (OtherComp :type "PrimitiveComponent Object Reference") (OtherBodyIndex :type Integer))
  ;[1 1 1] Left Hand Overlap End
  (set `self.Actor Left` null)
  (`self.Deactivate Left Hand IK`))

(event `self.Right.OnComponentEndOverlap`
  (params (OverlappedComponent :type "PrimitiveComponent Object Reference") (OtherActor :type "Actor Object Reference") (OtherComp :type "PrimitiveComponent Object Reference") (OtherBodyIndex :type Integer))
  ;[1 1 1] Right Hand Overlap End
  (set `self.Actor Right` null)
  (`self.Deactivate Right Hand IK`))

(event `Activate Left Hand IK`
  ;[1 1 1] Smoothly move hand toward / away from near object
  (if (not (`TimelineComponent.IsPlaying` (`self.Hand IK L Activate`)))
    (if (not (> (`self.Hand IK Left`) 0.0))
      (bind (_direction _hand_ik) (`Timeline|Hand IK L Activate` :!via `PlayFromStart`)
        (:`Update`
          (set `self.Hand IK Left` _hand_ik))))
    (message `/Game/ImmersiveTemplate/Blueprints/Immersive_Interface.IK Left Hand Activate` (`SkeletalMeshComponent.GetAnimInstance` (`Character.Mesh` (`self.As Character`))) (`self.Left Hand Location`) _hand_ik)))

(event `Deactivate Left Hand IK`
  ;[1 1 1] Smoothly move hand toward / away from near object
  (if (`TimelineComponent.IsPlaying` (`self.Hand IK L Deactivate`))
    _
    (elif (not (== (`self.Hand IK Left`) 0.0))
      (bind (_direction _hand_ik) (`Timeline|Hand IK L Deactivate` :!via `PlayFromStart`)
        (:`Update`
          (bind _output_get (set `self.Hand IK Left` _hand_ik))
          (message `/Game/ImmersiveTemplate/Blueprints/Immersive_Interface.IK Left Hand Activate` (`SkeletalMeshComponent.GetAnimInstance` (`Character.Mesh` (`self.As Character`))) (`self.Left Hand Location`) _output_get))
        (:`Finished`
          (set `self.Hand IK Left` 0.0))))))

(event `Activate Right Hand IK`
  ;[1 1 1] Smoothly move hand toward / away from near object
  (if (not (`TimelineComponent.IsPlaying` (`self.Hand IK R Activate`)))
    (if (not (> (`self.Hand IK Right`) 0.0))
      (bind (_direction _hand_ik) (`Timeline|Hand IK R Activate` :!via `PlayFromStart`)
        (:`Update`
          (bind _output_get (set `self.Hand IK Right` _hand_ik)))))
    (message `/Game/ImmersiveTemplate/Blueprints/Immersive_Interface.IK Right Hand Activate` (`SkeletalMeshComponent.GetAnimInstance` (`Character.Mesh` (`self.As Character`))) (`self.Right Hand Location`) _output_get)))

(event `Deactivate Right Hand IK`
  ;[1 1 1] Smoothly move hand toward / away from near object
  (if (`TimelineComponent.IsPlaying` (`self.Hand IK R Deactivate`))
    _
    (elif (not (== (`self.Hand IK Right`) 0.0))
      (bind (_direction _hand_ik) (`Timeline|Hand IK R Deactivate` :!via `PlayFromStart`)
        (:`Update`
          (bind _output_get (set `self.Hand IK Right` _hand_ik))
          (message `/Game/ImmersiveTemplate/Blueprints/Immersive_Interface.IK Right Hand Activate` (`SkeletalMeshComponent.GetAnimInstance` (`Character.Mesh` (`self.As Character`))) (`self.Right Hand Location`) _output_get))
        (:`Finished`
          (set `self.Hand IK Right` 0.0))))))

(fn `UserConstructionScript`
  (`SceneComponent.SetHiddenInGame` (`self.Right`) (not (`self.👾 Debug?`)) false)
  (`SceneComponent.SetHiddenInGame` (`self.Left`) (not (`self.👾 Debug?`)) false))